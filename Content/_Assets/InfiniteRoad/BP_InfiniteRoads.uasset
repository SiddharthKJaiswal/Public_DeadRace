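; BP_InfiniteRoads is the controller that builds an endless road out of chained tiles populated with zombies.
; SpawnSection lays a random run of default tiles, then a random left or right turn.
; SpawnTile places each tile at the stored transform, registers itself as its controller and takes the tile's end point as the next spawn.
; Zombies spawn at jittered mob points offset from that updated point and are recorded on the tile.
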(fn `Spawn Mobs`
  (params (SpawnPos :type "Vector Structure"))
  (returns (Mob :type "/Game/_Project/Pawns/BP_Zombie Object Reference"))
  (bind _returnvalue (`AIBlueprintHelperLibrary.SpawnAIFromClass` "/Game/_Project/Pawns/BP_Zombie.BP_Zombie_C" null SpawnPos (`KismetMathLibrary.MakeRotator` 0.0 0.0 (`KismetMathLibrary.RandomFloatInRange` -90.0 90.0)) false null))
  (bind _asbp_zombie (cast `/Game/_Project/Pawns/BP_Zombie` _returnvalue))
  (return _asbp_zombie))

(fn `SpawnSection`
  (for _ (range (+ (`KismetMathLibrary.RandomIntegerInRange` 1 5) 1))
    (`self.SpawnTile` null))
  (`self.SpawnTile` (select `bool` (`KismetMathLibrary.RandomBool`) :`false` "/Game/_Assets/InfiniteRoad/BP_Road_Turn_Left.BP_Road_Turn_Left_C" :`true` "/Game/_Assets/InfiniteRoad/BP_Road_Turn_Right.BP_Road_Turn_Right_C" :!type "Actor Class Reference"))
  (return))

(fn `SpawnTile`
  (params (TileToSpawn :type "Actor Class Reference"))
  (bind _returnvalue (`KismetMathLibrary.RandomFloatInRange` -150.0 150.0))
  (bind _returnvalue_2 (`|SpawnActorFromClass` TileToSpawn (`self.NextSpawnPoint`) "AlwaysSpawn" "MultiplyWithRoot" null null))
  (bind _asbp_road_base (cast `/Game/_Assets/InfiniteRoad/BP_Road_Base` _returnvalue_2))
  (set `/Game/_Assets/InfiniteRoad/BP_Road_Base.Controller` self _asbp_road_base)
  (set `self.NextSpawnPoint` (`SceneComponent.K2_GetComponentToWorld` (`/Game/_Assets/InfiniteRoad/BP_Road_Base.NextSpawnPoint` _asbp_road_base)))
  (for _array_element (`/Game/_Assets/InfiniteRoad/BP_Road_Base.MobSpawnPoints` _asbp_road_base)
    (bind _mob (`self.Spawn Mobs` (+ (`KismetMathLibrary.MakeVector` (+ (.x _array_element) _returnvalue) (+ (.y _array_element) _returnvalue) (.z _array_element)) (.location (`self.NextSpawnPoint`)))))
    (`KismetArrayLibrary.Array_Add` (`/Game/_Assets/InfiniteRoad/BP_Road_Base.Mobs` _asbp_road_base) _mob)))

(fn `UserConstructionScript`)