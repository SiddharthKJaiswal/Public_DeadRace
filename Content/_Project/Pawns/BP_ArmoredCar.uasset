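; Player-driven armored car that runs over and shoots zombies, with a HUD for speed, distance, kills and health.
; Enhanced Input drives vehicle movement, material-based brake lights and a pitch-clamped platform that follows the camera's control rotation.
; KillBox overlaps ragdoll zombies and count kills, while body hits from other zombies trigger their attack and update health.
; A looping timer fires bullets from the rifle's muzzle socket, and Escape toggles the pause menu.
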(event `self.ReceiveBeginPlay`
  ;[1 1 1] Initialization
  (bind _asplayer_controller (cast `PlayerController` (`self.GetController`)))
  (set `self.MyPlayerController` _asplayer_controller)
  (bind _returnvalue (pcsubsystem `EnhancedInputLocalPlayerSubsystem` _asplayer_controller))
  (`/Engine/EditorBlueprintResources/StandardMacros.IsValid` _returnvalue
    (:`Is Valid`
      (`EnhancedInputSubsystemInterface.AddMappingContext` _returnvalue "/Game/_Project/Inputs/IMC_Vehicle.IMC_Vehicle" 0 (struct))
      (bind _returnvalue_2 (`|CreateWidget` "/Game/_Project/UserInterface/WBP_Overlay.WBP_Overlay_C" _asplayer_controller))
      (bind _output_get (set `self.OverlayWidget` _returnvalue_2))
      (`UserWidget.AddToViewport` _output_get 0))))

(event `EnhancedInput|/Game/_Project/Inputs/Vehicle/IA_Look`
  (params (ActionValue :type "Vector2D Structure") (ElapsedSeconds :type "Float (double-precision)") (TriggeredSeconds :type "Float (double-precision)") (InputAction :type "InputAction Object Reference" :default "/Game/_Project/Inputs/Vehicle/IA_Look.IA_Look"))
  (bind (_x _y) (`KismetMathLibrary.BreakVector2D` ActionValue))
  (bind (_returnvalue_roll _returnvalue_pitch _returnvalue_yaw) (`KismetMathLibrary.BreakRotator` (`self.GetControlRotation`)))
  ;[1 1 1] Camera Controls
  (:`Triggered`
    (`self.AddControllerYawInput` _x)
    (`self.AddControllerPitchInput` _y)
    (`SceneComponent.K2_SetWorldRotation` (`self.Platform`) (`KismetMathLibrary.MakeRotator` 0.0 (`KismetMathLibrary.ClampAngle` _returnvalue_pitch 335.0 25.0) _returnvalue_yaw) false false)))

(event `EnhancedInput|/Game/_Project/Inputs/Vehicle/IA_Accelerate`
  (params (ActionValue :type "Float (double-precision)") (ElapsedSeconds :type "Float (double-precision)") (TriggeredSeconds :type "Float (double-precision)") (InputAction :type "InputAction Object Reference" :default "/Game/_Project/Inputs/Vehicle/IA_Accelerate.IA_Accelerate"))
  ;[1 1 1] Vehicle Controls
  (:`Triggered`
    (`ChaosVehicleMovementComponent.SetThrottleInput` (`self.VehicleMovementComponent`) ActionValue :!label _label)
    (`/Engine/EditorBlueprintResources/StandardMacros.DoOnce` false
      (:`Completed`
        (`MaterialInstanceDynamic.SetScalarParameterValue` (`self.Mesh Material`) "BrakeLightPower" 15.0))))
  (:`Completed`
    (goto _label)))

(event `EnhancedInput|/Game/_Project/Inputs/Vehicle/IA_Decelerate`
  (params (ActionValue :type "Float (double-precision)") (ElapsedSeconds :type "Float (double-precision)") (TriggeredSeconds :type "Float (double-precision)") (InputAction :type "InputAction Object Reference" :default "/Game/_Project/Inputs/Vehicle/IA_Decelerate.IA_Decelerate"))
  ;[1 1 1] Vehicle Controls
  (:`Triggered`
    (`self.BrakeLights` true)
    (`ChaosVehicleMovementComponent.SetBrakeInput` (`self.VehicleMovementComponent`) ActionValue :!label _label_2))
  (:`Completed`
    (`self.BrakeLights` false)
    (goto _label_2)))

(event `EnhancedInput|/Game/_Project/Inputs/Vehicle/IA_HandBrake`
  (params (ActionValue :type Boolean) (ElapsedSeconds :type "Float (double-precision)") (TriggeredSeconds :type "Float (double-precision)") (InputAction :type "InputAction Object Reference" :default "/Game/_Project/Inputs/Vehicle/IA_HandBrake.IA_HandBrake"))
  ;[1 1 1] Vehicle Controls
  (:`Triggered`
    (`self.BrakeLights` ActionValue :!label _label_3)
    (`ChaosVehicleMovementComponent.SetHandbrakeInput` (`self.VehicleMovementComponent`) ActionValue))
  (:`Completed`
    (goto _label_3)))

(event `EnhancedInput|/Game/_Project/Inputs/Vehicle/IA_Steer`
  (params (ActionValue :type "Float (double-precision)") (ElapsedSeconds :type "Float (double-precision)") (TriggeredSeconds :type "Float (double-precision)") (InputAction :type "InputAction Object Reference" :default "/Game/_Project/Inputs/Vehicle/IA_Steer.IA_Steer"))
  ;[1 1 1] Vehicle Controls
  (:`Triggered`
    (`ChaosVehicleMovementComponent.SetSteeringInput` (`self.VehicleMovementComponent`) ActionValue :!label _label_4))
  (:`Completed`
    (goto _label_4)))

(event `self.ReceiveTick`
  (params (DeltaSeconds :type "Float (single-precision)"))
  (bind _returnvalue (* (`KismetMathLibrary.Abs` (`ChaosVehicleMovementComponent.GetForwardSpeed` (`self.VehicleMovementComponent`))) 0.036))
  ;[1 1 1] Update UI
  (if (> _returnvalue 1.0)
    (`/Game/_Project/UserInterface/WBP_Overlay.UpdateSpeed` (`self.OverlayWidget`) (`KismetMathLibrary.FTrunc` _returnvalue))
    (`/Game/_Project/UserInterface/WBP_Overlay.UpdateDistance` (`self.OverlayWidget`) (`KismetMathLibrary.FTrunc` (* (`GameplayStatics.GetWorldDeltaSeconds`) _returnvalue)))))

(event `self.KillBox.OnComponentBeginOverlap`
  (params (OverlappedComponent :type "PrimitiveComponent Object Reference") (OtherActor :type "Actor Object Reference") (OtherComp :type "PrimitiveComponent Object Reference") (OtherBodyIndex :type Integer) (bFromSweep :type Boolean) (SweepResult :type "HitResult Structure (by ref)"))
  ;[1 1 1] Character
  (bind _asbp_zombie (cast `/Game/_Project/Pawns/BP_Zombie` OtherActor))
  (if (`/Game/_Project/Pawns/BP_Zombie.CanHit` _asbp_zombie)
    (set `self.Struck` _asbp_zombie)
    (`/Game/_Project/Pawns/BP_Zombie.Ragdoll` _asbp_zombie)
    (`/Game/_Project/UserInterface/WBP_Overlay.UpdateKillCount` (`self.OverlayWidget`))
    (`PrimitiveComponent.SetCollisionEnabled` (`Character.CapsuleComponent` _asbp_zombie) "NoCollision")
    (set `/Game/_Project/Pawns/BP_Zombie.CanHit` false _asbp_zombie)))

(event `self.Mesh.OnComponentHit`
  (params (HitComponent :type "PrimitiveComponent Object Reference") (OtherActor :type "Actor Object Reference") (OtherComp :type "PrimitiveComponent Object Reference") (NormalImpulse :type "Vector Structure") (Hit :type "HitResult Structure (by ref)"))
  ;[1 1 1] Character
  (bind _asbp_zombie (cast `/Game/_Project/Pawns/BP_Zombie` OtherActor))
  (if (not (== _asbp_zombie (`self.Struck`)))
    (`/Game/_Project/Pawns/BP_Zombie.AttackPlayer` _asbp_zombie)
    (`/Game/_Project/UserInterface/WBP_Overlay.UpdateHealth` (`self.OverlayWidget`) false)))

(event `EnhancedInput|/Game/_Project/Inputs/Vehicle/IA_Shoot`
  (params (ActionValue :type Boolean) (ElapsedSeconds :type "Float (double-precision)") (TriggeredSeconds :type "Float (double-precision)") (InputAction :type "InputAction Object Reference" :default "/Game/_Project/Inputs/Vehicle/IA_Shoot.IA_Shoot"))
  ;[1 1 1] Gun Controls
  (:`Started`
    (bind _returnvalue (`KismetSystemLibrary.K2_SetTimerDelegate` (delegate `Shoot`) 0.1 true))
    (set `self.ShootHandle` _returnvalue))
  (:`Completed`
    (`KismetSystemLibrary.K2_ClearAndInvalidateTimerHandle` (`self.ShootHandle`))))

(event `Shoot`
  (bind _returnvalue (`SceneComponent.GetSocketTransform` (`self.Assault_Rifle_A`) "MuzzleFlash" "RTS_World"))
  ;[1 1 1] Gun Controls
  (`|SpawnActorFromClass` "/Game/_Project/Props/BP_Bullet.BP_Bullet_C" _returnvalue "AlwaysSpawn" "MultiplyWithRoot" null self null)
  (`GameplayStatics.SpawnEmitterAtLocation` "/Game/_Assets/Props/Gun/P_AssaultRifle_MuzzleFlash.P_AssaultRifle_MuzzleFlash" (.location _returnvalue) (struct) (1.0 1.0 1.0) true "AutoRelease"))

(event `Key|Escape`
  (params (Key :type "Key Structure"))
  (:`Pressed`
    (`/Engine/EditorBlueprintResources/StandardMacros.FlipFlop`
      (:`A`
        (set `PlayerController.bShowMouseCursor` true (`self.MyPlayerController`))
        (`self.PauseWidget`
          (:`then`
            _)
          (:`else`
            (bind _returnvalue (`|CreateWidget` "/Game/_Project/UserInterface/WBP_Pause.WBP_Pause_C" (`self.MyPlayerController`)))
            (set `self.PauseWidget` _returnvalue)))
        (`UserWidget.AddToViewport` (`self.PauseWidget`) 0)
        (`WidgetBlueprintLibrary.SetInputMode_GameAndUIEx` (`self.MyPlayerController`) (`self.PauseWidget`)))
      (:`B`
        (set `PlayerController.bShowMouseCursor` false (`self.MyPlayerController`))
        (`Widget.RemoveFromParent` (`self.PauseWidget`))
        (`WidgetBlueprintLibrary.SetInputMode_GameOnly` (`self.MyPlayerController`))))))

(fn `BrakeLights`
  (params (IsBraking :type Boolean))
  (`MaterialInstanceDynamic.SetScalarParameterValue` (`self.Mesh Material`) "BrakeLightPower" (`KismetMathLibrary.SelectFloat` 200.0 15.0 IsBraking)))

(fn `UserConstructionScript`
  (bind _returnvalue (`PrimitiveComponent.CreateDynamicMaterialInstance` (`self.Mesh`) 0 null "None"))
  (set `self.Mesh Material` _returnvalue))