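; BP_Zombie is an enemy character that chases and lunges at the armored car.
; When PawnSensing sees the car, it moves within range via AIMoveTo, then, on success or failure, disables mesh collision and launches itself toward it.
; AttackPlayer plays a bite montage and destroys the actor when playback ends.
; Ragdoll switches the mesh to physics simulation and destroys the actor after a short delay.
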(event `self.PawnSensing.OnSeePawn`
  (params (Pawn :type "Pawn Object Reference"))
  (bind _asbp_armored_car (cast `/Game/_Project/Pawns/BP_ArmoredCar` Pawn))
  (`|AIMoveTo` self (0.0 0.0 0.0) _asbp_armored_car 350.0 true
    (:`OnSuccess`
      _)
    (:`OnFail`
      _))
  (`self.LaunchCharacter` (0.0 0.0 10.0))
  (`PrimitiveComponent.SetCollisionEnabled` (`self.Mesh`) "NoCollision")
  (`self.LaunchCharacter` (* (`KismetMathLibrary.GetDirectionUnitVector` (`self.K2_GetActorLocation`) (`self.K2_GetActorLocation` _asbp_armored_car)) (1000.0 1000.0 10.0))))

(event `AttackPlayer`
  (`|PlayMontage` (`self.Mesh`) "/Game/_Assets/Pawns/Humanoid/Zombie/Animations/AM_Bite.AM_Bite"
    (:`OnCompleted`
      _)
    (:`OnBlendOut`
      _)
    (:`OnInterrupted`
      _))
  (`self.K2_DestroyActor`))

(event `Ragdoll`
  (`PrimitiveComponent.SetCollisionEnabled` (`self.CapsuleComponent`) "NoCollision")
  (`PrimitiveComponent.SetCollisionObjectType` (`self.Mesh`) "ECC_PhysicsBody")
  (`PrimitiveComponent.SetCollisionEnabled` (`self.Mesh`) "QueryAndPhysics")
  (`SkeletalMeshComponent.SetAllBodiesSimulatePhysics` (`self.Mesh`) true)
  (`KismetSystemLibrary.Delay` 2.0)
  (`self.K2_DestroyActor`))

(fn `UserConstructionScript`)